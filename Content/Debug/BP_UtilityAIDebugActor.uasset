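; Debug actor that shows the Utility AI state of an observed actor through a widget component.
; GetObservedActor resolves the target from the ObservedActor variable, falling back to parent actor, attach parent, instigator, then owner.
; After a zero-second delay on BeginPlay, it finds the FtsUtilityAIComponent on that actor's AI controller and passes it to the WB_UtilityAIDebug widget.
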(event EventBeginPlay
  (bind _returnvalue (CallFunction|GetObservedActor))
  (bind _returnvalue_2 (AI|GetAIController _returnvalue))
  (bind _returnvalue_3 (Actor|GetComponentbyClass _returnvalue_2 "/Script/FtsUtilityAI.FtsUtilityAIComponent"))
  (Utilities|FlowControl|Delay 0.0)
  (Utilities|IsValid _returnvalue_3
    (:Is%20Valid
      (bind _aswb_utility_aidebug (Utilities|Casting|CastToWB_UtilityAIDebug (UserInterface|GetUserWidgetObject (Variables|Default|GetWidget))))
      (Default|SetUtilityComponent _aswb_utility_aidebug _returnvalue_3))))

(event Collision|EventActorBeginOverlap
  (params (OtherActor :type Actor%20Object%20Reference)))

(event EventTick
  (params (DeltaSeconds :type Float%20%28single-precision%29)))

(fn ConstructionScript)

(fn GetObservedActor
  (bind _returnvalue (Actor|GetAttachParentActor))
  (bind _returnvalue_2 (Actor|GetParentActor))
  (bind _returnvalue_3 (Game|GetInstigator))
  (Utilities|FlowControl|Sequence
    (:then_0
      (bind _observedactor (Variables|Default|GetObservedActor)
        (:then
          (return _observedactor))
        (:else)))
    (:then_1
      (Utilities|IsValid _returnvalue_2
        (:Is%20Valid
          (return _returnvalue_2))))
    (:then_2
      (Utilities|IsValid _returnvalue
        (:Is%20Valid
          (return _returnvalue))))
    (:then_3
      (Utilities|IsValid _returnvalue_3
        (:Is%20Valid
          (return _returnvalue_3))))
    (:then_4
      (return (Components|GetOwner)))))