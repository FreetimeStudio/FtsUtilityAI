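; BP_FtsSplinePathAiTarget is an AI target actor that moves along a spline path, staying ahead of a following actor.
; BeginPlay takes the spline from PathActor and seeds the position with the input key closest to the follower, later treated as distance along the spline.
; Each tick advances that position by any shortfall below StayAheadDistance, never backward, wraps it at the spline length and snaps the actor's transform there.
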(event Custom|InitializeSplinePosition
  (Variables|Default|SetCurrentSplinePosition (Class|SplineComponent|FindInputKeyClosesttoWorldLocation (Variables|Default|GetSplinePath) (Transformation|GetActorLocation (Variables|Default|GetFollowingActor)))))

(event Custom|SetSplinePath
  (params (NewSplinePath :type Spline%20Component%20Object%20Reference))
  (Variables|Default|SetSplinePath NewSplinePath)
  (CallFunction|InitializeSplinePosition)
  (CallFunction|UpdateLocation))

(event Custom|UpdateLocation
  (Transformation|SetActorTransform (Spline|GetTransformatDistanceAlongSpline (Variables|Default|GetSplinePath) (Variables|Default|GetCurrentSplinePosition) "World" false)))

(event Custom|UpdateSplinePosition
  (Variables|Default|SetCurrentSplinePosition (Math|Float|%(Float) (+ (Variables|Default|GetCurrentSplinePosition) (Math|Float|Max(Float) (* (- (Transformation|GetDistanceTo (Variables|Default|GetFollowingActor)) (Variables|Default|GetStayAheadDistance)) -1.0) 0.0)) (Spline|GetSplineLength (Variables|Default|GetSplinePath)))))

(event EventTick
  (params (DeltaSeconds :type Float%20%28single-precision%29))
  (CallFunction|UpdateSplinePosition)
  (CallFunction|UpdateLocation))

(event EventBeginPlay
  (bind _pathactor (Variables|Default|GetPathActor)
    (:then
      (CallFunction|SetSplinePath (Actor|GetComponentbyClass _pathactor "/Script/Engine.SplineComponent")))
    (:else)))

(fn ConstructionScript)