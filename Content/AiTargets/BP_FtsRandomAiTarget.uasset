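; An AI target actor that repeatedly jumps to random locations.
; On BeginPlay it stores its origin, then loops ChooseNewLocation with a random delay drawn from ChangeDelay.
; Each move offsets a random 3D direction by a distance from DistanceRange, measured from the origin if ConstrainToOrigin is set, otherwise from its current location.
; Moves are unswept, and the UpdateLocation event is empty.
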(event Custom|UpdateLocation)

(event EventBeginPlay
  (bind _changedelay (Variables|Default|GetChangeDelay))
  (Variables|Default|SetOrigin (Transformation|GetActorLocation))
  (CallFunction|ChooseNewLocation :!label _label)
  (Utilities|FlowControl|Delay (Math|Random|RandomFloatinRange (.min _changedelay) (.max _changedelay)))
  (goto _label))

(fn ConstructionScript)

(fn ChooseNewLocation
  (bind _distancerange (Variables|Default|GetDistanceRange))
  (LocalVariables|SetRange (Math|Random|RandomFloatinRange (.min _distancerange) (.max _distancerange)))
  (Transformation|SetActorLocation (+ (Math|Vector|ClampVectorSize (Math|Random|RandomUnitVector) (LocalVariables|GetRange) (LocalVariables|GetRange)) (select (Variables|Default|GetbConstrainToOrigin) (Variables|Default|GetOrigin) (Transformation|GetActorLocation))) false false))