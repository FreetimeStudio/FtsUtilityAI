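; Patrol AI target actor that moves itself along a list of patrol points as a patrolling actor reaches it.
; It snaps to the current point's location on BeginPlay.
; Tick checks the patrolling actor's distance to the target; within the reach threshold, it waits a switch delay, advances the index with modulo wrap-around, then jumps to the next point.
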(event Custom|UpdateLocation
  (Transformation|SetActorLocation (Transformation|GetActorLocation (Utilities|Array|Get(acopy) (Variables|Default|GetPatrolPoints) (Variables|Default|GetCurrentPatrolPointIndex))) false false))

(event EventTick
  (params (DeltaSeconds :type Float%20%28single-precision%29))
  (if (<= (Transformation|GetDistanceTo (Variables|Default|GetPatrollingActor)) (Variables|Default|GetPointReachedDistance))
    (Utilities|FlowControl|Delay (Variables|Default|GetPointSwitchDelay))
    (bind _result (Math|Integer|IncrementInt (Variables|Default|GetCurrentPatrolPointIndex))
      (:%20%20
        (Variables|Default|SetCurrentPatrolPointIndex (Math|Integer|%(Integer) _result (Utilities|Array|Length (Variables|Default|GetPatrolPoints))))
        (CallFunction|UpdateLocation)))))

(event EventBeginPlay
  (CallFunction|UpdateLocation))

(fn ConstructionScript)